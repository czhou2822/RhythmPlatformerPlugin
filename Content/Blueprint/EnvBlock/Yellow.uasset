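; Yellow environment block that BP_Dude can smash when its color matches, and that hurts the player otherwise.
; Box1 overlap stores the player, and Tick destroys the block with a bump sound and force feedback once color and a required player state both match.
; Leaving the box while the block is intact calls the player's DamageSyatem for a small amount of damage.
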(event `self.ReceiveBeginPlay`
  (set `self.MyColor` "NewEnumerator0"))

(event `self.Box1.OnComponentBeginOverlap`
  (params (OverlappedComponent :type "PrimitiveComponent Object Reference") (OtherActor :type "Actor Object Reference") (OtherComp :type "PrimitiveComponent Object Reference") (OtherBodyIndex :type Integer) (bFromSweep :type Boolean) (SweepResult :type "HitResult Structure (by ref)"))
  (bind _asbp_dude (cast `/Game/Blueprint/BP_Dude` OtherActor))
  (set `self.bIsOverlapping` true)
  (set `self.Player` _asbp_dude))

(event `self.Box1.OnComponentEndOverlap`
  (params (OverlappedComponent :type "PrimitiveComponent Object Reference") (OtherActor :type "Actor Object Reference") (OtherComp :type "PrimitiveComponent Object Reference") (OtherBodyIndex :type Integer))
  (bind _asbp_dude (cast `/Game/Blueprint/BP_Dude` OtherActor))
  (if (not (`self.bIsDestoryed`))
    (`KismetSystemLibrary.PrintString` "Hurt")
    (`/Game/Blueprint/BP_Dude.DamageSyatem` _asbp_dude 0.1)
    (set `self.bIsOverlapping` false)))

(event `self.ReceiveTick`
  (params (DeltaSeconds :type "Float (single-precision)"))
  (bind _player (`self.Player`))
  (`|ExecutionSequence`
    (:`then_0`
      (`KismetSystemLibrary.PrintString` (`KismetStringLibrary.Conv_BoolToString` (`self.bIsDestoryed`)) false)
      (if (`self.bIsOverlapping`)
        (if (== (`KismetMathLibrary.And_IntInt` (`KismetMathLibrary.Conv_BoolToInt` (`|EnumEquality` (`/Game/Blueprint/BP_Dude.Color` _player) (`self.MyColor`))) (`KismetMathLibrary.Conv_BoolToInt` (`|EnumEquality` (`/Game/Blueprint/BP_Dude.state` _player) "NewEnumerator7"))) 1)
          (set `self.bIsDestoryed` true)
          (`GameplayStatics.PlaySoundAtLocation` "/Game/Sound/SFX/Bump.Bump" (`self.K2_GetActorLocation`) (struct) 1.0 1.0 0.0 null null null)
          (`self.K2_DestroyActor`)
          (`PlayerController.K2_ClientPlayForceFeedback` (`GameplayStatics.GetPlayerController` 0) "/Game/NewForceFeedbackEffect.NewForceFeedbackEffect" "None" false false false))))))

(fn `UserConstructionScript`)