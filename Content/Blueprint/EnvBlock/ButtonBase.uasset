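; ButtonBase is a base button actor that tests the player's color and action state and reports success or failure to the game mode.
; BeginPlay caches the BP_Dude player, and CheckButton passes only when its color matches the button's and its action state matches a fixed value.
; EndButton notifies RPPGameMode or RPPTutorialGameMode, always as success in the tutorial, then destroys the button.
; Nothing here calls CheckButton or EndButton.
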(event `self.ReceiveBeginPlay`
  (bind _asbp_dude (cast `/Game/Blueprint/PlayerCharacter/BP_Dude` (`GameplayStatics.GetPlayerCharacter` 0)))
  (set `self.PlayerCharacterBase` _asbp_dude))

(fn `CheckButton`
  (returns (ReturnValue :type Boolean))
  (locals (NewLocalVar_0 :type "/Game/Blueprint/PlayerCharacter/BP_Dude Object Reference"))
  (bind _playercharacterbase (`self.PlayerCharacterBase`))
  (bind _issame (`self.CheckPlayerColor` _playercharacterbase))
  (bind _issame_2 (`self.CheckPlayerActionState` _playercharacterbase))
  (return (and _issame _issame_2)))

(fn `CheckPlayerActionState`
  (params (NewParam :type "/Game/Blueprint/PlayerCharacter/BP_Dude Object Reference"))
  (returns (IsSame :type Boolean))
  (bind _actionstate (`/Game/Blueprint/PlayerCharacter/BP_Dude.ActionState` NewParam))
  (`KismetSystemLibrary.PrintString` (`KismetStringLibrary.Concat_StrStr` "PlayerState: " (`|GetEnumeratorNameAsString` _actionstate)) false true (struct :`G` 0.66 :`B` 1.0 :`A` 1.0) 0.1)
  (return (`|EnumEquality` _actionstate "NewEnumerator11")))

(fn `CheckPlayerColor`
  (params (NewParam :type "/Game/Blueprint/PlayerCharacter/BP_Dude Object Reference"))
  (returns (IsSame :type Boolean))
  (bind _playercolor (`/Game/Blueprint/PlayerCharacter/BP_Dude.PlayerColor` NewParam))
  (bind _buttoncolor (`self.ButtonColor`))
  (`KismetSystemLibrary.PrintString` (`KismetStringLibrary.Concat_StrStr` "PlayerColor: " (`|GetEnumeratorNameAsString` _playercolor) " ButtonColor: " (`|GetEnumeratorNameAsString` _buttoncolor)) false true (struct :`G` 0.66 :`B` 1.0 :`A` 1.0) 0.1)
  (return (== _playercolor _buttoncolor)))

(fn `EndButton`
  (params (IsSuccess :type Boolean))
  (bind _returnvalue (`GameplayStatics.GetGameMode`))
  (bind _asrppgame_mode (cast `/Game/RPPGameMode` _returnvalue)
    (:`then`
      (if IsSuccess
        (`/Game/RPPGameMode.ButtonSuccess` _asrppgame_mode self)
        (else
          (`/Game/RPPGameMode.ButtonFailed` _asrppgame_mode self)))
      (`self.K2_DestroyActor`))
    (:`CastFailed`
      (bind _asrpptutorial_game_mode (cast `/Game/Tutorial/RPPTutorialGameMode` _returnvalue))
      (if true
        (`/Game/Tutorial/RPPTutorialGameMode.ButtonSuccess` _asrpptutorial_game_mode self)
        (else
          (`/Game/Tutorial/RPPTutorialGameMode.ButtonFailed` _asrpptutorial_game_mode self)))
      (`self.K2_DestroyActor`))))

(fn `UserConstructionScript`)