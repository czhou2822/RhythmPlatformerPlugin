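; Colored Paper2D sprite block that runs a button check when the player's BP_Dude overlaps it, tinted red, blue, black or green in the construction script.
; In the required action state, overlap starts a fast looping timer that polls CheckButton until success calls EndButton(true).
; Any other state fails immediately with EndButton(false).
; Older destroy, damage and out-of-bound logic remains in the graph but never runs.
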(event `self.ReceiveBeginPlay`
  (`parent.ReceiveBeginPlay`))

(event `self.Box1.OnComponentBeginOverlap`
  (params (OverlappedComponent :type "PrimitiveComponent Object Reference") (OtherActor :type "Actor Object Reference") (OtherComp :type "PrimitiveComponent Object Reference") (OtherBodyIndex :type Integer) (bFromSweep :type Boolean) (SweepResult :type "HitResult Structure (by ref)"))
  (bind _asbp_dude (cast `/Game/Blueprint/PlayerCharacter/BP_Dude` OtherActor))
  (if (`|EnumEquality` (`/Game/Blueprint/PlayerCharacter/BP_Dude.ActionState` _asbp_dude) "NewEnumerator12")
    (bind _returnvalue (`KismetSystemLibrary.K2_SetTimer` null "CheckButtonTick" 0.01 true))
    (set `self.TIckHandler` _returnvalue)
    (set `self.IsOverlapping` true)
    (else
      (`self.EndButton` false))))

(event `self.Box1.OnComponentEndOverlap`
  (params (OverlappedComponent :type "PrimitiveComponent Object Reference") (OtherActor :type "Actor Object Reference") (OtherComp :type "PrimitiveComponent Object Reference") (OtherBodyIndex :type Integer)))

(event `self.ReceiveTick`
  (params (DeltaSeconds :type "Float (single-precision)")))

(fn `CheckButtonTick`
  (`KismetSystemLibrary.PrintString` (`KismetStringLibrary.Concat_StrStr` "Button: " (`KismetSystemLibrary.GetDisplayName` self) " active") false true (struct :`G` 0.66 :`B` 1.0 :`A` 1.0) 0.1)
  (bind _returnvalue (`self.CheckButton`))
  (if _returnvalue
    (`self.EndButton` true)
    (`KismetSystemLibrary.K2_ClearAndInvalidateTimerHandle` (`self.TIckHandler`))))

(fn `UserConstructionScript`
  (switch `/Game/Blueprint/E_Color` (`self.MyColorBase`)
    (:`NewEnumerator0`
      (set `self.NewColor` (struct :`R` 1.0 :`A` 1.0)))
    (:`NewEnumerator1`
      (set `self.NewColor` (struct :`B` 1.0 :`A` 1.0)))
    (:`NewEnumerator2`
      (set `self.NewColor` (struct :`A` 1.0)))
    (:`NewEnumerator3`
      (set `self.NewColor` (struct :`G` 1.0 :`A` 1.0))))
  (`PaperSpriteComponent.SetSpriteColor` (`self.PaperSprite`) (`self.NewColor`)))