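; Hold-button obstacle for a runner game that awards points while the player holds through a colored, spline-length segment.
; Construction sizes the hit box, sprite and fill-bar widget from two spline points and tints the sprite by ButtonColor.
; When BP_Dude overlaps in the required action state, a looping timer polls CheckButton, adds GameMode points and fills the bar.
; Hold duration derives from length over running speed; EndButton reports completion or failure.
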(event `self.ReceiveBeginPlay`
  (`parent.ReceiveBeginPlay`)
  (`KismetSystemLibrary.Delay` 0.2)
  (bind _asumg_hold_button_fillup (cast `/Game/Blueprint/EnvBlock/UMG_HoldButtonFillup` (`WidgetComponent.GetUserWidgetObject` (`self.FillUpBar`))))
  (set `self.HoldButtonFillup` _asumg_hold_button_fillup)
  (bind _asrppgame_mode (cast `/Game/RPPGameMode` (`GameplayStatics.GetGameMode`)))
  (set `self.HoldDuration` (/ (`self.TotalLength`) (`/Game/RPPGameMode.PlayerRunningSpeed` _asrppgame_mode))))

(event `self.ReceiveTick`
  (params (DeltaSeconds :type "Float (single-precision)")))

(event `self.TestHitBox.OnComponentBeginOverlap`
  (params (OverlappedComponent :type "PrimitiveComponent Object Reference") (OtherActor :type "Actor Object Reference") (OtherComp :type "PrimitiveComponent Object Reference") (OtherBodyIndex :type Integer) (bFromSweep :type Boolean) (SweepResult :type "HitResult Structure (by ref)"))
  (if (not (`KismetSystemLibrary.K2_IsValidTimerHandle` (`self.ActiveHandler`)))
    (bind _asbp_dude (cast `/Game/Blueprint/PlayerCharacter/BP_Dude` OtherActor))
    (if (`|EnumEquality` (`/Game/Blueprint/PlayerCharacter/BP_Dude.ActionState` _asbp_dude) "NewEnumerator12")
      (bind _returnvalue (`KismetSystemLibrary.K2_SetTimer` null "CheckButtonTick" 0.01 true))
      (set `self.ActiveHandler` _returnvalue)
      (`SceneComponent.SetVisibility` (`self.FillUpBar`) true false)
      (else
        (`self.EndButton` false)))))

(event `self.TestHitBox.OnComponentEndOverlap`
  (params (OverlappedComponent :type "PrimitiveComponent Object Reference") (OtherActor :type "Actor Object Reference") (OtherComp :type "PrimitiveComponent Object Reference") (OtherBodyIndex :type Integer))
  (cast `/Game/Blueprint/PlayerCharacter/BP_Dude` OtherActor)
  (`KismetSystemLibrary.K2_ClearAndInvalidateTimerHandle` (`self.ActiveHandler`))
  (if (not (>= (`self.Progress`) 1.0))
    (`self.EndButton` false)))

(fn `AddToPoint`)

(fn `CheckButtonTick`
  (bind _holdduration (`self.HoldDuration`))
  (bind _returnvalue (`self.CheckButton`))
  (if _returnvalue
    (bind _asrppgame_mode (cast `/Game/RPPGameMode` (`GameplayStatics.GetGameMode`)))
    (`/Game/RPPGameMode.AddHoldButtonPoint` _asrppgame_mode 1)
    (bind _output_get (set `self.HoldValue` (+ (`self.HoldValue`) 0.01)))
    (bind _returnvalue_2 (/ _output_get _holdduration))
    (`KismetSystemLibrary.PrintString` (`KismetStringLibrary.Concat_StrStr` "Value： " (`KismetStringLibrary.Conv_DoubleToString` _output_get) " Duration" (`KismetStringLibrary.Conv_DoubleToString` _holdduration) " Percentage: " (`KismetStringLibrary.Conv_DoubleToString` _returnvalue_2)) false)
    (bind _output_get_2 (set `self.Progress` _returnvalue_2))
    (`ProgressBar.SetPercent` (`/Game/Blueprint/EnvBlock/UMG_HoldButtonFillup.HoldProgressBar` (`self.HoldButtonFillup`)) (* _output_get_2 1.05))
    (if (>= (`self.Progress`) 1.0)
      (`self.EndButton` true))))

(fn `MakeRankingBox`
  (bind _papersprite (`self.PaperSprite`))
  (bind _spline (`self.Spline`))
  (bind _fillupbar (`self.FillUpBar`))
  (bind (_returnvalue_x _returnvalue_y) (`KismetMathLibrary.BreakVector2D` (`WidgetComponent.GetDrawSize` _fillupbar)))
  (bind _returnvalue (- (`SplineComponent.GetLocationAtSplinePoint` _spline 1 "Local") (`SplineComponent.GetLocationAtSplinePoint` _spline 0 "Local")))
  (bind (_returnvalue_x_2 _returnvalue_y_2 _returnvalue_z) (`KismetMathLibrary.BreakVector` (/ _returnvalue 2.0)))
  (bind _x (.x _returnvalue))
  (set `self.TotalLength` _x)
  ;[1 1 1] CollisionBox
  (bind _returnvalue_2 (`AddComponent|NODE_AddBoxComponent-0` :`RelativeTransform` (`KismetMathLibrary.MakeTransform` (`KismetMathLibrary.MakeVector` _returnvalue_x_2 _returnvalue_y_2 _returnvalue_z))))
  (bind _output_get (set `self.TestHitBox` _returnvalue_2))
  (`BoxComponent.SetBoxExtent` _output_get (`KismetMathLibrary.MakeVector` (+ _returnvalue_x_2 (`self.Tollerance`)) 1.0 64.0) true)
  (`SceneComponent.SetHiddenInGame` (`self.TestHitBox`) false false)
  ;[1 1 1] Papersprite
  (`SceneComponent.K2_SetRelativeLocation` _papersprite (`KismetMathLibrary.MakeVector` _returnvalue_x_2 _returnvalue_y_2 _returnvalue_z) false false)
  (`SceneComponent.SetRelativeScale3D` _papersprite (`KismetMathLibrary.MakeVector` (/ _returnvalue_x_2 64.0) 1.0 1.0))
  (`WidgetComponent.SetDrawSize` _fillupbar (`KismetMathLibrary.MakeVector2D` (* _x 3.82) _returnvalue_y)))

(fn `SetMyColor`
  (locals (NewColor :type "LinearColor Structure"))
  (switch `/Game/Blueprint/E_Color` (`self.ButtonColor`)
    (:`NewEnumerator0`
      (set `local.NewColor` (struct :`R` 1.0 :`A` 1.0)))
    (:`NewEnumerator1`
      (set `local.NewColor` (struct :`B` 1.0 :`A` 1.0)))
    (:`NewEnumerator2`
      (set `local.NewColor` (struct :`A` 1.0)))
    (:`NewEnumerator3`
      (set `local.NewColor` (struct :`G` 1.0 :`A` 1.0))))
  (`PaperSpriteComponent.SetSpriteColor` (`self.PaperSprite`) (`local.NewColor`)))

(fn `UserConstructionScript`
  (`self.MakeRankingBox`)
  (`self.SetMyColor`))