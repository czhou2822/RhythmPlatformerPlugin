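; Spline pad actor that carries the player along its spline once a BP_Dude overlaps its sphere.
; On BeginPlay it reads the running speed from BP_PluginManager and sets spline duration to the end points' world X distance divided by that speed.
; After activation, Tick advances a timer and moves the character to the spline location at that time until the duration runs out.
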(event `self.ReceiveBeginPlay`
  (`|ExecutionSequence`
    (:`then_0`
      (bind _outactors (`GameplayStatics.GetAllActorsOfClass` "/Game/Sound/BP_PluginManager.BP_PluginManager_C"))
      (set `self.PlayerRunningSpeed` (`MySecondPluginManager.RunningSpeed` (`|GetArrayItem` _outactors))))
    (:`then_1`
      (`self.Set Spline DurationBP`))))

(event `self.ReceiveTick`
  (params (DeltaSeconds :type "Float (single-precision)"))
  (if (`self.IsActive`)
    (if (<= (`self.Timer`) (`SplineComponent.Duration` (`self.SplineComp`)))
      (bind _output_get (set `self.Timer` (+ DeltaSeconds (`self.Timer`))))
      (`self.K2_SetActorLocation` (`self.PlayerCharacter`) (`SplineComponent.GetLocationAtTime` (`self.SplineComp`) _output_get "World" false) false false))))

(event `self.Sphere.OnComponentBeginOverlap`
  (params (OverlappedComponent :type "PrimitiveComponent Object Reference") (OtherActor :type "Actor Object Reference") (OtherComp :type "PrimitiveComponent Object Reference") (OtherBodyIndex :type Integer) (bFromSweep :type Boolean) (SweepResult :type "HitResult Structure (by ref)"))
  (bind _asbp_dude (cast `/Game/Blueprint/PlayerCharacter/BP_Dude` OtherActor))
  (set `self.IsActive` true)
  (set `self.PlayerCharacter` _asbp_dude))

(fn `Set Spline DurationBP`
  (bind _splinecomp (`self.SplineComp`))
  (bind _returnvalue_x (`KismetMathLibrary.BreakVector` (`SplineComponent.GetLocationAtSplinePoint` (`self.SplineComp`) 0 "World")))
  (bind _returnvalue_x_2 (`KismetMathLibrary.BreakVector` (`SplineComponent.GetLocationAtSplinePoint` _splinecomp (- (`SplineComponent.GetNumberOfSplinePoints` _splinecomp) 1) "World")))
  (bind _returnvalue (/ (- _returnvalue_x_2 _returnvalue_x) (`self.PlayerRunningSpeed`)))
  (set `SplineComponent.Duration` _returnvalue (`self.SplineComp`))
  (`KismetSystemLibrary.PrintString` (`KismetStringLibrary.Concat_StrStr` "spline duration: " (`KismetStringLibrary.Conv_DoubleToString` _returnvalue)) false))

(fn `UserConstructionScript`)